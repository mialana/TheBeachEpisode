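; BP_GameModeSkate is the game mode for skating, which extends the ground by spawning BP_Ground actors end to end.
; On BeginPlay it finds the level's initial ground, reads its world-space generation location and rotation, and fires OnGenerateNextGround, or prints an error if none exists.
; That event spawns the next segment there, caches the new segment's generation point for the following spawn, and prints the result.
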(event EventBeginPlay
  (bind _returnvalue (Actor|GetActorOfClass "/Game/TheBeachEpisode/Core/Interactables/BP_Ground.BP_Ground_C"))
  (Utilities|IsValid _returnvalue
    (:Is%20Valid
      (Variables|Default|SetNextGenerationLocation (.GenerationLocation (Default|GetGenerationDataWorldSpace _returnvalue)))
      (Variables|Default|SetNextGenerationRotation (.GenerationRotation (Default|GetGenerationDataWorldSpace _returnvalue)))
      (Class|TheBeachEpisodeGameModeInterface|OnGenerateNextGround))
    (:Is%20Not%20Valid
      (Development|PrintString "No initial ground actor found in level."))))

(event EventTick
  (params (DeltaSeconds :type Float%20%28single-precision%29)))

(event EventOnGenerateNextGround
  (bind _returnvalue (Game|SpawnActorfromClass "/Game/TheBeachEpisode/Core/Interactables/BP_Ground.BP_Ground_C" (Math|Transform|MakeTransform (Variables|Default|GetNextGenerationLocation) (Variables|Default|GetNextGenerationRotation) "1.000000,1.000000,1.000000") "Undefined" "MultiplyWithRoot" 0 0))
  (Variables|Default|SetNextGenerationLocation (.GenerationLocation (Default|GetGenerationDataWorldSpace _returnvalue)))
  (Variables|Default|SetNextGenerationRotation (.GenerationRotation (Default|GetGenerationDataWorldSpace _returnvalue)))
  (Development|PrintText (Utilities|Text|FormatText "New ground actor generated at <{Location}> with rotation <{Rotation}>." (Utilities|Text|ToText(String) (Variables|Default|GetNextGenerationLocation)) (Utilities|Text|ToText(String) (Variables|Default|GetNextGenerationRotation)))))

(fn ConstructionScript)